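; BP_DodgeChallenger is a player-driven vehicle Blueprint for a Dodge Challenger.
; On BeginPlay it caches the player controller and adds the IMC_VehicleInputMap Enhanced Input mapping context.
; Input actions feed throttle, brake/reverse, steering, gear shifts and handbrake straight into the vehicle movement component, clearing held inputs on release.
; Look input drives controller yaw and pitch for mouse look.
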(event `EnhancedInput|/Game/Blueprints/Input/IA_Throttle`
  (params (ActionValue :type "Float (double-precision)") (ElapsedSeconds :type "Float (double-precision)") (TriggeredSeconds :type "Float (double-precision)") (InputAction :type "InputAction Object Reference" :default "/Game/Blueprints/Input/IA_Throttle.IA_Throttle"))
  ;[0.04483 0.15 0.02783 0.5] Forward, Reverse/Brake & Steering
  (:`Triggered`
    (`ChaosVehicleMovementComponent.SetThrottleInput` (`self.VehicleMovementComponent`) ActionValue))
  (:`Completed`
    (`ChaosVehicleMovementComponent.SetThrottleInput` (`self.VehicleMovementComponent`) 0.0)))

(event `EnhancedInput|/Game/Blueprints/Input/IA_ReverseBrake`
  (params (ActionValue :type "Float (double-precision)") (ElapsedSeconds :type "Float (double-precision)") (TriggeredSeconds :type "Float (double-precision)") (InputAction :type "InputAction Object Reference" :default "/Game/Blueprints/Input/IA_ReverseBrake.IA_ReverseBrake"))
  ;[0.04483 0.15 0.02783 0.5] Forward, Reverse/Brake & Steering
  (:`Triggered`
    (`ChaosVehicleMovementComponent.SetBrakeInput` (`self.VehicleMovementComponent`) ActionValue))
  (:`Canceled`
    (`ChaosVehicleMovementComponent.SetBrakeInput` (`self.VehicleMovementComponent`) 0.0 :!label _label))
  (:`Completed`
    (goto _label)))

(event `self.ReceiveBeginPlay`
  (bind _asplayer_controller (cast `PlayerController` (`self.GetController`)))
  (bind _output_get (set `self._playerController` _asplayer_controller))
  (message `EnhancedInputSubsystemInterface.AddMappingContext` (pcsubsystem `EnhancedInputLocalPlayerSubsystem` _output_get) "/Game/Blueprints/Input/IMC_VehicleInputMap.IMC_VehicleInputMap" 0 (struct)))

(event `EnhancedInput|/Game/Blueprints/Input/IA_Steer`
  (params (ActionValue :type "Float (double-precision)") (ElapsedSeconds :type "Float (double-precision)") (TriggeredSeconds :type "Float (double-precision)") (InputAction :type "InputAction Object Reference" :default "/Game/Blueprints/Input/IA_Steer.IA_Steer"))
  ;[0.04483 0.15 0.02783 0.5] Forward, Reverse/Brake & Steering
  (:`Triggered`
    (`ChaosVehicleMovementComponent.SetSteeringInput` (`self.VehicleMovementComponent`) ActionValue))
  (:`Completed`
    (`ChaosVehicleMovementComponent.SetSteeringInput` (`self.VehicleMovementComponent`) 0.0)))

(event `EnhancedInput|/Game/Blueprints/Input/IA_ShiftGearUp`
  (params (ActionValue :type Boolean) (ElapsedSeconds :type "Float (double-precision)") (TriggeredSeconds :type "Float (double-precision)") (InputAction :type "InputAction Object Reference" :default "/Game/Blueprints/Input/IA_ShiftGearUp.IA_ShiftGearUp"))
  ;[0.04483 0.15 0.02783 0.5] Gear up & down
  (:`Started`
    (`ChaosVehicleMovementComponent.SetChangeUpInput` (`self.VehicleMovementComponent`) ActionValue)))

(event `EnhancedInput|/Game/Blueprints/Input/IA_ShiftGearDown`
  (params (ActionValue :type Boolean) (ElapsedSeconds :type "Float (double-precision)") (TriggeredSeconds :type "Float (double-precision)") (InputAction :type "InputAction Object Reference" :default "/Game/Blueprints/Input/IA_ShiftGearDown.IA_ShiftGearDown"))
  ;[0.04483 0.15 0.02783 0.5] Gear up & down
  (:`Started`
    (`ChaosVehicleMovementComponent.SetChangeDownInput` (`self.VehicleMovementComponent`) ActionValue)))

(event `EnhancedInput|/Game/Blueprints/Input/IA_HandBrake`
  (params (ActionValue :type Boolean) (ElapsedSeconds :type "Float (double-precision)") (TriggeredSeconds :type "Float (double-precision)") (InputAction :type "InputAction Object Reference" :default "/Game/Blueprints/Input/IA_HandBrake.IA_HandBrake"))
  (bind _vehiclemovementcomponent (`self.VehicleMovementComponent`))
  ;[0.04483 0.15 0.02783 0.5] Handbrake
  (:`Triggered`
    (`ChaosVehicleMovementComponent.SetHandbrakeInput` _vehiclemovementcomponent true))
  (:`Canceled`
    (`ChaosVehicleMovementComponent.SetHandbrakeInput` _vehiclemovementcomponent false :!label _label_2))
  (:`Completed`
    (goto _label_2)))

(event `EnhancedInput|/Game/Blueprints/Input/IA_Look`
  (params (ActionValue :type "Vector2D Structure") (ElapsedSeconds :type "Float (double-precision)") (TriggeredSeconds :type "Float (double-precision)") (InputAction :type "InputAction Object Reference" :default "/Game/Blueprints/Input/IA_Look.IA_Look"))
  (bind (_x _y) (`KismetMathLibrary.BreakVector2D` ActionValue))
  ;[0.04483 0.15 0.02783 0.5] Mouse look
  (:`Triggered`
    (`PlayerController.AddYawInput` (`self._playerController`) _x)
    (`PlayerController.AddPitchInput` (`self._playerController`) _y)))

(fn `UserConstructionScript`)