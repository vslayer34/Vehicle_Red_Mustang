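; Player-drivable Red Dodge vehicle pawn with Enhanced Input controls and a spring arm camera.
; BeginPlay caches the spring arm's default length and socket offset and adds the vehicle mapping context.
; Input actions feed steering, throttle, brake and handbrake to the vehicle movement component, while look input rotates the controller.
; Two seconds after look input completes, a Timeline lerps arm length and offset toward defaults, printing a debug string each update.
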(event `self.ReceiveBeginPlay`
  (bind _springarm (`self.SpringArm`))
  (`|ExecutionSequence`
    (:`then_0`
      (set `self._defaultTargetArmLength` (`SpringArmComponent.TargetArmLength` _springarm))
      (set `self._defaultSocketOffset` (`SpringArmComponent.SocketOffset` _springarm)))
    (:`then_1`
      (bind _asplayer_controller (cast `PlayerController` (`self.GetController`)))
      (bind _output_get (set `self._playerController` _asplayer_controller))
      (`EnhancedInputSubsystemInterface.AddMappingContext` (pcsubsystem `EnhancedInputLocalPlayerSubsystem` _output_get) "/Game/Blueprints/Input/IMC_VehicleInputMap.IMC_VehicleInputMap" 0 (struct)))))

(event `EnhancedInput|/Game/Blueprints/Input/IA_Steer`
  (params (ActionValue :type "Float (double-precision)") (ElapsedSeconds :type "Float (double-precision)") (TriggeredSeconds :type "Float (double-precision)") (InputAction :type "InputAction Object Reference" :default "/Game/Blueprints/Input/IA_Steer.IA_Steer"))
  (bind _vehiclemovementcomponent (`self.VehicleMovementComponent`))
  (:`Triggered`
    (`ChaosVehicleMovementComponent.SetSteeringInput` _vehiclemovementcomponent ActionValue))
  (:`Canceled`
    (`ChaosVehicleMovementComponent.SetSteeringInput` _vehiclemovementcomponent 0.0 :!label _label))
  (:`Completed`
    (goto _label)))

(event `EnhancedInput|/Game/Blueprints/Input/IA_Throttle`
  (params (ActionValue :type "Float (double-precision)") (ElapsedSeconds :type "Float (double-precision)") (TriggeredSeconds :type "Float (double-precision)") (InputAction :type "InputAction Object Reference" :default "/Game/Blueprints/Input/IA_Throttle.IA_Throttle"))
  (bind _vehiclemovementcomponent (`self.VehicleMovementComponent`))
  (:`Started`
    (`ChaosVehicleMovementComponent.SetThrottleInput` _vehiclemovementcomponent ActionValue))
  (:`Completed`
    (`ChaosVehicleMovementComponent.SetThrottleInput` _vehiclemovementcomponent 0.0)))

(event `EnhancedInput|/Game/Blueprints/Input/IA_HandBrake`
  (params (ActionValue :type Boolean) (ElapsedSeconds :type "Float (double-precision)") (TriggeredSeconds :type "Float (double-precision)") (InputAction :type "InputAction Object Reference" :default "/Game/Blueprints/Input/IA_HandBrake.IA_HandBrake"))
  (bind _vehiclemovementcomponent (`self.VehicleMovementComponent`))
  (:`Triggered`
    (`ChaosVehicleMovementComponent.SetHandbrakeInput` _vehiclemovementcomponent ActionValue))
  (:`Canceled`
    (`ChaosVehicleMovementComponent.SetHandbrakeInput` _vehiclemovementcomponent false :!label _label_2))
  (:`Completed`
    (goto _label_2)))

(event `EnhancedInput|/Game/Blueprints/Input/IA_ReverseBrake`
  (params (ActionValue :type "Float (double-precision)") (ElapsedSeconds :type "Float (double-precision)") (TriggeredSeconds :type "Float (double-precision)") (InputAction :type "InputAction Object Reference" :default "/Game/Blueprints/Input/IA_ReverseBrake.IA_ReverseBrake"))
  (bind _vehiclemovementcomponent (`self.VehicleMovementComponent`))
  (:`Started`
    (`ChaosVehicleMovementComponent.SetBrakeInput` _vehiclemovementcomponent ActionValue))
  (:`Canceled`
    (`ChaosVehicleMovementComponent.SetBrakeInput` _vehiclemovementcomponent 0.0 :!label _label_3))
  (:`Completed`
    (goto _label_3)))

(event `EnhancedInput|/Game/Blueprints/Input/IA_Look`
  (params (ActionValue :type "Vector2D Structure") (ElapsedSeconds :type "Float (double-precision)") (TriggeredSeconds :type "Float (double-precision)") (InputAction :type "InputAction Object Reference" :default "/Game/Blueprints/Input/IA_Look.IA_Look"))
  (bind __playercontroller (`self._playerController`))
  (:`Triggered`
    (`PlayerController.AddYawInput` __playercontroller ActionValue_X)
    (`PlayerController.AddPitchInput` __playercontroller ActionValue_Y))
  (:`Completed`
    (`KismetSystemLibrary.Delay` 2.0)
    (bind (_direction _floattrack) (`Timeline|Timeline` :`NewTime` 1.0 :!via `PlayFromStart`)
      (:`Update`
        (`KismetSystemLibrary.PrintString` "Hello" true true (struct :`G` 0.66 :`B` 1.0 :`A` 1.0) 502.0)
        (`self.ResetSpringArmPosition` _floattrack)))))

(fn `ResetSpringArmPosition`
  (params (ratio :type "Float (double-precision)"))
  (bind _springarm (`self.SpringArm`))
  (set `SpringArmComponent.TargetArmLength` (`KismetMathLibrary.Lerp` (`SpringArmComponent.TargetArmLength` _springarm) (`self._defaultTargetArmLength`) ratio) _springarm)
  (set `SpringArmComponent.SocketOffset` (`KismetMathLibrary.VLerp` (`SpringArmComponent.SocketOffset` (`self.SpringArm`)) (`self._defaultSocketOffset`) (`local.ratio`)) _springarm))

(fn `UserConstructionScript`)